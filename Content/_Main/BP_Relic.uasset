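; BP_Relic is an interactable relic that offers the player a one-time ability unlock.
; Its trigger shows a widget and registers the relic with BP_OurPlayer as interactable while in range.
; Interact opens WBP_Decision and blocks movement input until NotAccepted or Decision closes it.
; Decision marks the relic accepted, calls AbilityUnlocked on GM_MainGame and destroys the trigger after a short delay.
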(event OnComponentBeginOverlap(Trigger)
  (params (OverlappedComponent :type Primitive%20Component%20Object%20Reference) (OtherActor :type Actor%20Object%20Reference) (OtherComp :type Primitive%20Component%20Object%20Reference) (OtherBodyIndex :type Integer) (bFromSweep :type Boolean) (SweepResult :type Hit%20Result%20Structure%20%28by%20ref%29))
  (if (Actor|ActorHasTag OtherActor "Player")
    (CallFunction|PlayerinRange)
    (bind _asbp_our_player (Utilities|Casting|CastToBP_OurPlayer OtherActor))
    (bind _output_get (Variables|Default|SetAs%20BP%20Our%20Player _asbp_our_player))
    (Variables|/Game/_Main/Player/BP_OurPlayer.BP_OurPlayer_C|SetCan%20Interact? _output_get true)
    (Variables|/Game/_Main/Player/BP_OurPlayer.BP_OurPlayer_C|SetCurrentRelic (Variables|Default|GetAs%20BP%20Our%20Player) self)))

(event OnComponentEndOverlap(Trigger)
  (params (OverlappedComponent :type Primitive%20Component%20Object%20Reference) (OtherActor :type Actor%20Object%20Reference) (OtherComp :type Primitive%20Component%20Object%20Reference) (OtherBodyIndex :type Integer))
  (if (Actor|ActorHasTag OtherActor "Player")
    (CallFunction|PlayerLeftRange)
    (bind _asbp_our_player (Utilities|Casting|CastToBP_OurPlayer OtherActor))
    (bind _output_get (Variables|Default|SetAs%20BP%20Our%20Player _asbp_our_player))
    (Variables|/Game/_Main/Player/BP_OurPlayer.BP_OurPlayer_C|SetCan%20Interact? _output_get false)))

(event Custom|Player%20In%20Range
  (Rendering|SetVisibility (Variables|Default|GetWidget) true false))

(event Custom|Player%20Left%20Range
  (Rendering|SetVisibility (Variables|Default|GetWidget) false false))

(event Custom|Decision
  (if (not (Variables|Default|GetIs%20Accepted?))
    (Variables|Default|SetIs%20Accepted? true)
    (bind _asgm_main_game (Utilities|Casting|CastToGM_MainGame (Game|GetGameMode)))
    (Utilities|IsValid _asgm_main_game
      (:Is%20Valid
        (Default|AbilityUnlocked _asgm_main_game)
        (Widget|RemovefromParent (Variables|Default|GetDecisionRef))
        (Variables|Default|SetDecisionRef 0)
        (Variables|/Game/_Main/Player/BP_OurPlayer.BP_OurPlayer_C|SetIsInteracting? (Variables|Default|GetAs%20BP%20Our%20Player) false)
        (Input|SetIgnoreMoveInput (Game|GetPlayerController 0) false)
        (Utilities|FlowControl|Delay 0.2)
        (Components|DestroyComponent (Variables|Default|GetTrigger))))
    (else
      (Development|PrintString "this relic already absorbed"))))

(event Custom|NotAccepted
  (bind _decisionref (Variables|Default|GetDecisionRef)
    (:then
      (Widget|RemovefromParent _decisionref)
      (Variables|Default|SetDecisionRef 0)
      (Variables|/Game/_Main/Player/BP_OurPlayer.BP_OurPlayer_C|SetIsInteracting? (Variables|Default|GetAs%20BP%20Our%20Player) false)
      (Input|SetIgnoreMoveInput (Game|GetPlayerController 0) false))
    (:else)))

(event EventBeginPlay)

(event Collision|EventActorBeginOverlap
  (params (OtherActor :type Actor%20Object%20Reference)))

(event EventTick
  (params (DeltaSeconds :type Float%20%28single-precision%29)))

(event EventInteract
  (bind _returnvalue (Game|GetPlayerController 0))
  (Development|PrintString "interacted with relic")
  (if (not (Variables|Default|GetIs%20Accepted?))
    (bind _returnvalue_2 (UserInterface|CreateWidget "/Game/_Main/WBP_Decision.WBP_Decision_C" _returnvalue))
    (bind _output_get (Variables|Default|SetDecisionRef _returnvalue_2))
    (UserInterface|Viewport|AddtoViewport _output_get 0)
    (Input|SetIgnoreMoveInput _returnvalue true)))

(fn ConstructionScript)