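; GM_MainGame is the main game mode, which handles ability unlocks for the player character.
; On BeginPlay it caches the BP_OurPlayer reference and resets an unlocked-ability counter.
; AbilityUnlocked increments the counter, then matches the current relic's AbilityToBeUnlocked to call the player's agile, air dash, air or jump ability function.
; An unmatched ability only prints a setup reminder.
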(event Custom|AbilityUnlocked
  (bind _as_bp_our_player (Variables|Default|GetAs%20BP%20Our%20Player))
  (bind _as_bp_our_player_2 (Variables|Default|GetAs%20BP%20Our%20Player))
  (bind _currentrelic (Variables|/Game/_Main/Player/BP_OurPlayer.BP_OurPlayer_C|GetCurrentRelic _as_bp_our_player))
  (Math|Integer|IncrementInt (Variables|Default|GetAbilities%20Unlocked)
    (:%20%20
      (if (== (Variables|/Game/_Main/Blueprints/BaseClass/BP_Relic.BP_Relic_C|GetAbilityToBeUnlocked _currentrelic) (Variables|Default|GetAgileAbility))
        (Default|AgileAbility _as_bp_our_player_2)
        (elif (== (Variables|/Game/_Main/Blueprints/BaseClass/BP_Relic.BP_Relic_C|GetAbilityToBeUnlocked _currentrelic) (Variables|Default|GetDashAbility))
          (Default|AirDashAbility _as_bp_our_player_2)
          (elif (== (Variables|/Game/_Main/Blueprints/BaseClass/BP_Relic.BP_Relic_C|GetAbilityToBeUnlocked _currentrelic) (Variables|Default|GetAirAbility))
            (Default|AirAbility _as_bp_our_player_2)
            (elif (== (Variables|/Game/_Main/Blueprints/BaseClass/BP_Relic.BP_Relic_C|GetAbilityToBeUnlocked _currentrelic) (Variables|Default|GetJumpAbility))
              (Default|JumpAbility _as_bp_our_player_2)
              (else
                (Development|PrintString "Set up ability Unlock")))))))))

(event EventBeginPlay
  (bind _asbp_our_player (Utilities|Casting|CastToBP_OurPlayer (Game|GetPlayerCharacter 0)))
  (Variables|Default|SetAs%20BP%20Our%20Player _asbp_our_player)
  (Variables|Default|SetAbilities%20Unlocked 0))

(event EventTick
  (params (DeltaSeconds :type Float%20%28single-precision%29)))

(fn ConstructionScript)