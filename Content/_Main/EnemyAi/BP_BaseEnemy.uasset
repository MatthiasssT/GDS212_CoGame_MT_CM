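; BP_BaseEnemy is an enemy character base with health, a simple state variable, directional hit reactions and attack movement.
; AnyDamage subtracts health, then either calls the empty PeformDeath or uses the BP_DT_Main damage type to pick a hit montage, setting state before playing it.
; AddAttackForce restarts a timeline that moves the actor along its forward vector with a swept location lerp, and StopAttackForce halts it.
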(event Custom|AddAttackForce
  (params (Distance :type Float%20%28double-precision%29))
  (bind _returnvalue (Transformation|GetActorLocation))
  ;[1 1 1] Hit Force (moveEnemy)
  (CallFunction|StopAttackForce)
  (if (!= Distance 0.0)
    (bind _alpha (Timeline|Timeline PlayFromStart)
      (:Update
        (Transformation|SetActorLocation (Math|Vector|Lerp(Vector) _returnvalue (+ _returnvalue (* (Transformation|GetActorForwardVector) Distance)) _alpha) true false)))))

(event Custom|StopAttackForce
  (bind _returnvalue (Transformation|GetActorLocation))
  ;[1 1 1] Hit Force (moveEnemy)
  (bind _alpha (Timeline|Timeline Stop)
    (:Update
      (Transformation|SetActorLocation (Math|Vector|Lerp(Vector) _returnvalue (+ _returnvalue (* (Transformation|GetActorForwardVector) (stale Custom|AddAttackForce Distance))) _alpha) true false))))

(event Game|Damage|EventAnyDamage
  (params (Damage :type Float%20%28single-precision%29) (DamageType :type Damage%20Type%20Object%20Reference) (InstigatedBy :type Controller%20Object%20Reference) (DamageCauser :type Actor%20Object%20Reference))
  ;[1 1 1] Enemy takes Damage
  (bind _output_get (Variables|Stats|SetHealth (- (Variables|Stats|GetHealth) Damage)))
  (if (> _output_get 0.0)
    (bind _asbp_dt_main (Utilities|Casting|CastToBP_DT_Main DamageType))
    (Utilities|IsValid (DamageTaken|GetHitMontage (Variables|/Game/_Main/DamageType/BP_DT_Main.BP_DT_Main_C|GetDamgeType _asbp_dt_main))
      (:Is%20Valid
        (State|SetState "NewEnumerator4")
        (Animation|PlayAnimMontage (DamageTaken|GetHitMontage (Variables|/Game/_Main/DamageType/BP_DT_Main.BP_DT_Main_C|GetDamgeType _asbp_dt_main)) 1.0 "None"))
      (:Is%20Not%20Valid
        (Development|PrintString "enemy hit reaction is not valid")))
    (else
      ;[1 1 1] if Health below 0 then call death function
      (DamageTaken|PeformDeath))))

(fn ConstructionScript)

(fn PeformDeath)

(fn GetHitMontage
  (params (DamageType :type E_DamageTypes%20Enum :default "NewEnumerator0"))
  (switch Utilities|FlowControl|Switch|SwitchonE_DamageTypes DamageType
    (:NewEnumerator0
      (return 0))
    (:NewEnumerator1
      (return (Variables|DamageTaken|GetHit%20R%20ANIM)))
    (:NewEnumerator2
      (return (Variables|DamageTaken|GetHit%20L%20ANIM)))
    (:NewEnumerator3
      (return (Variables|DamageTaken|GetHit%20M%20ANIM)))
    (:NewEnumerator4
      (return (Variables|DamageTaken|GetHit%20D%20ANIM)))
    (:NewEnumerator5
      (return (Variables|DamageTaken|GetHit%20B%20ANIM)))))

(fn SetState
  (params (NewState :type E_States%20Enum :default "NewEnumerator0"))
  (if (Utilities|Enum|NotEqual(Enum) NewState (Variables|State|GetCurrentState))
    (Variables|State|SetCurrentState NewState)))

(fn GetState
  (return (Variables|State|GetCurrentState)))

(fn IsStateEqualtoAny
  (params (States%20to%20check :type Array%20of%20E_States%20Enums :default "NewEnumerator0"))
  (return (Utilities|Array|ContainsItem States%20to%20check (Variables|State|GetCurrentState))))